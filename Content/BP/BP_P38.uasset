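; BP_P38 is a player-controlled P-38 plane pawn that flies constantly forward, steered by pitch and roll input scaled by delta time.
; Fire spawns BP_Rocket at a body socket, BombDrop spawns at the Drop socket with no class set, and Boost raises MaxSpeed to the movement component's Acceleration value while held.
; BeginPlay registers both propellers with BPRotateSceneComponent for spinning, leaving the local PropellerRotate function uncalled.
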(event `self.ReceiveTick`
  (params (DeltaSeconds :type "Float (single-precision)"))
  ;[1 1 1] 단순한 전진
  (`self.AddMovementInput` (`self.GetActorForwardVector`)))

(event `InputAction|Fire`
  (params (Key :type "Key Structure"))
  ;[1 1 1] 공격(로켓발사)
  (:`Pressed`
    (`|SpawnActorFromClass` "/Game/BP/BP_Rocket.BP_Rocket_C" (`SceneComponent.GetSocketTransform` (`self.SM_P38_Body`) "SpawnRocket" "RTS_World") "Undefined" "MultiplyWithRoot" null null)))

(event `InputAction|BombDrop`
  (params (Key :type "Key Structure"))
  ;[1 1 1] 폭격
  (:`Pressed`
    (`|SpawnActorFromClass` "/Game/BP/BP_Rocket_Drop.BP_Rocket_Drop_C" (`SceneComponent.GetSocketTransform` (`self.SM_P38_Body`) "Drop" "RTS_World") "Undefined" "MultiplyWithRoot" null null)))

(event `InputAxis|Pitch`
  (params (AxisValue :type "Float (single-precision)"))
  ;[1 1 1] 비행기 몸체 회전
  (`self.K2_AddActorLocalRotation` (`KismetMathLibrary.MakeRotator` 0.0 (* AxisValue (`GameplayStatics.GetWorldDeltaSeconds`) (`self.PlaneRotateSpeed`)))))

(event `InputAction|Boost`
  (params (Key :type "Key Structure"))
  (bind _floatingpawnmovement (`self.FloatingPawnMovement`))
  ;[1 1 1] 속도 부스트(LeftShift)
  (:`Pressed`
    (set `FloatingPawnMovement.MaxSpeed` (`FloatingPawnMovement.Acceleration` _floatingpawnmovement) _floatingpawnmovement))
  (:`Released`
    (set `FloatingPawnMovement.MaxSpeed` 500.0 _floatingpawnmovement)))

(event `InputAxis|Roll`
  (params (AxisValue :type "Float (single-precision)"))
  ;[1 1 1] 비행기 몸체 회전
  (`self.K2_AddActorLocalRotation` (`KismetMathLibrary.MakeRotator` (* AxisValue (`GameplayStatics.GetWorldDeltaSeconds`) (`self.PlaneRotateSpeed`)))))

(event `self.ReceiveBeginPlay`
  (bind _scenecomponents (`/Game/BP/BP_RotateSceneComponent.SceneComponents` (`self.BP_RotateSceneComponent`)))
  ;[1 1 1] 시작하면 BP RotateSceneComp에 씬컴포넌트 배열에 애들을 추가시켜준다.
  ; 배열에 들어가면 돌아감
  (`KismetArrayLibrary.Array_Add` _scenecomponents (`self.PropLeft`))
  (`KismetArrayLibrary.Array_Add` _scenecomponents (`self.PropRight`)))

(fn `PropellerRotate`
  (params (Where :type "SceneComponent Object Reference"))
  (`SceneComponent.K2_AddLocalRotation` Where (`KismetMathLibrary.MakeRotator` (* (`self.PropRotateValue`) (`GameplayStatics.GetWorldDeltaSeconds`))) false false))

(fn `UserConstructionScript`)